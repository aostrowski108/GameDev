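; BP_Enemy is an enemy actor that reacts to overlaps on its static mesh.
; Touching a BP_Projectile destroys both the projectile and the enemy, then adds one point to the player's Score.
; Touching a BP_Player applies fixed damage to player pawn 0 and leaves the enemy alive.
; It has no movement or Tick logic of its own.
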(event OnComponentBeginOverlap(StaticMesh)
  (params (OverlappedComponent :type Primitive%20Component%20Object%20Reference) (OtherActor :type Actor%20Object%20Reference) (OtherComp :type Primitive%20Component%20Object%20Reference) (OtherBodyIndex :type Integer) (bFromSweep :type Boolean) (SweepResult :type Hit%20Result%20Structure%20%28by%20ref%29))
  (if (Utilities|ClassIsChildOf (Utilities|GetClass OtherActor) "/Game/InfiniteMatrix/Blueprints/BP_Projectile.BP_Projectile_C")
    (Actor|DestroyActor OtherActor)
    (Actor|DestroyActor)
    (bind _asbp_player (Utilities|Casting|CastToBP_Player (Game|Player|GetPlayerPawn 0)))
    (Variables|/Game/InfiniteMatrix/Blueprints/BP_Player.BP_Player_C|SetScore _asbp_player (+ (Variables|/Game/InfiniteMatrix/Blueprints/BP_Player.BP_Player_C|GetScore _asbp_player) 1.0))
    (elif (Utilities|ClassIsChildOf (Utilities|GetClass OtherActor) "/Game/InfiniteMatrix/Blueprints/BP_Player.BP_Player_C")
      (bind _asbp_player_2 (Utilities|Casting|CastToBP_Player (Game|Player|GetPlayerPawn 0)))
      (Game|Damage|ApplyDamage _asbp_player_2 1e+01 0 0))))

(event EventBeginPlay)

(event Collision|EventActorBeginOverlap
  (params (OtherActor :type Actor%20Object%20Reference)))

(event EventTick
  (params (DeltaSeconds :type Float%20%28single-precision%29)))

(fn ConstructionScript)